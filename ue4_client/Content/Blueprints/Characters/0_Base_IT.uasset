(event `Key|R`
  (params (Key :type "Key Structure"))
  (:`Pressed`
    (bind _outactors (`GameplayStatics.GetAllActorsOfClass` "/Game/Blueprints/Gameplay/Devices/0_Base_Hackable.0_Base_Hackable_C"))
    (for _array_element _outactors
      (`/Game/Blueprints/Gameplay/GameplayPC.PerformRecover` (cast `/Game/Blueprints/Gameplay/GameplayPC` (`GameplayStatics.GetPlayerController` 0) :!pure true) _array_element))))

(event `Key|F`
  (params (Key :type "Key Structure"))
  (:`Pressed`
    (bind _outactors (`GameplayStatics.GetAllActorsOfClass` "/Game/Blueprints/Gameplay/Devices/0_Base_Hackable.0_Base_Hackable_C"))
    (for _array_element _outactors
      (`/Game/Blueprints/Gameplay/GameplayPC.PerformHack` (cast `/Game/Blueprints/Gameplay/GameplayPC` (`GameplayStatics.GetPlayerController` 0) :!pure true) _array_element))))

(event `Key|I`
  (params (Key :type "Key Structure"))
  (bind _asgameplay_pc (cast `/Game/Blueprints/Gameplay/GameplayPC` (`GameplayStatics.GetPlayerController` 0) :!pure true))
  (:`Pressed`
    (`/Game/Blueprints/Gameplay/GameplayPC.ScanDevices` _asgameplay_pc _asgameplay_pc)))

(fn `UserConstructionScript`
  (`parent.UserConstructionScript`))